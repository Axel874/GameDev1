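; Player character for a Mario-style side-view game, with axis-driven movement, a mouse-following Aim component and a tutorial widget shown at start.
; Jump launches the character, falling back to a limited hammer jump when Cube overlaps the GameState hammer's trigger and the hammer's idle time is within tolerance.
; Tick moves Aim and resets jump counters on the ground.
; Goomba overlaps reload the level; mushroom overlaps destroy the pickup and print a message.
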(event `self.ReceiveActorBeginOverlap`
  (params (OtherActor :type "Actor Object Reference"))
  (cast `/Game/Actors/Entities/BP_Goomba` OtherActor
    (:`then`
      (`self.HandleGoombaColission`))
    (:`CastFailed`
      (bind _asbp_mushroom (cast `/Game/Actors/Entities/BP_Mushroom` OtherActor))
      (`self.HandleMushroomCollision` _asbp_mushroom))))

(event `self.ReceiveBeginPlay`
  (bind _returnvalue (`|CreateWidget` "/Game/HUD/Tutorial.Tutorial_C"))
  (`UserWidget.AddToViewport` _returnvalue 0))

(event `self.ReceiveTick`
  (params (DeltaSeconds :type "Float (single-precision)"))
  (`self.UpdateCursor`)
  (`self.UpdateJumpCounter`))

(event `InputAction|JUMP`
  (params (Key :type "Key Structure"))
  (:`Pressed`
    (`self.HandleJump`)))

(event `InputAxis|MoveLeft`
  (params (AxisValue :type "Float (single-precision)"))
  (`self.AddMovementInput` (0.0 1.0 0.0) AxisValue))

(fn `HandleGoombaColission`
  (bind _returnvalue (`GameplayStatics.GetCurrentLevelName` true))
  (`GameplayStatics.OpenLevel` (`KismetStringLibrary.Conv_StringToName` _returnvalue)))

(fn `HandleJump`
  (if (`self.IsAllowedToJump`)
    (`self.LaunchCharacter` (`KismetMathLibrary.MakeVector` 0.0 0.0 (`self.jumpForce`)) false true)
    (`/Engine/EditorBlueprintResources/StandardMacros.IncrementInt` (`self.currentJumps`))
    (elif (`self.Is Allowed To Hammer Jump`)
      (`self.LaunchCharacter` (`KismetMathLibrary.MakeVector` 0.0 0.0 (`self.jumpForce`)) false true)
      (`/Engine/EditorBlueprintResources/StandardMacros.IncrementInt` (`self.currentHammerJumps`)))))

(fn `HandleMushroomCollision`
  (params (mushroom :type "/Game/Actors/Entities/BP_Mushroom Object Reference"))
  (`self.K2_DestroyActor` mushroom)
  (`KismetSystemLibrary.PrintString` "Mushroom pickup"))

(fn `Is Allowed To Hammer Jump`
  (returns (ReturnValue :type Boolean))
  (bind _asbp_mario_game_state (cast `/Game/GameModes/BP_MarioGameState` (`GameplayStatics.GetGameState`)))
  (bind _player_hammer (`/Game/GameModes/BP_MarioGameState.player Hammer` _asbp_mario_game_state))
  (return (and (< (`self.currentHammerJumps`) (`self.hammerJumps`)) (`PrimitiveComponent.IsOverlappingComponent` (`self.Cube`) (`/Game/Characters/BP_Hammer.JumpTrigger` _player_hammer)) (< (`/Game/Characters/BP_Hammer.timeIdle` _player_hammer) (`self.hammerJumpTolerance`)))))

(fn `UpdateCursor`
  (bind _aim (`self.aim`))
  (bind _returnvalue_x (`KismetMathLibrary.BreakVector` (`SceneComponent.K2_GetComponentLocation` _aim)))
  (bind _worldlocation (`PlayerController.DeprojectMousePositionToWorld` (`GameplayStatics.GetPlayerController` 0)))
  (`SceneComponent.K2_SetWorldLocation` _aim (`KismetMathLibrary.MakeVector` _returnvalue_x (.y _worldlocation) (.z _worldlocation)) false false))

(fn `UpdateJumpCounter`
  (if (`NavMovementComponent.IsMovingOnGround` (`self.CharacterMovement`))
    (set `self.currentJumps` 0)
    (set `self.currentHammerJumps` 0)))

(fn `UserConstructionScript`)