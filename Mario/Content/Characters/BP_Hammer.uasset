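; BP_Hammer is the player's boomerang-style thrown hammer, which registers itself as PlayerHammer in the Mario game state.
; An Idle/Outgoing/Incoming state drives Tick: it follows the player, flies toward the mouse on left click, or homes back, spinning while airborne.
; It turns back after a timeout or hitting an object, and player overlap resets it to idle.
; Directions come from normalized screen-space vectors mapped onto the Y-Z plane.
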(event OnComponentBeginOverlap(Cube)
  (params (OverlappedComponent :type Primitive%20Component%20Object%20Reference) (OtherActor :type Actor%20Object%20Reference) (OtherComp :type Primitive%20Component%20Object%20Reference) (OtherBodyIndex :type Integer) (bFromSweep :type Boolean) (SweepResult :type Hit%20Result%20Structure%20%28by%20ref%29))
  (bind _asbp_mario (Utilities|Casting|CastToBP_Mario OtherActor)
    (:then
      (CallFunction|HandlePlayerCollision _asbp_mario))
    (:CastFailed
      (CallFunction|HandleObjectCollision))))

(event EventBeginPlay
  (bind _asbp_mario_game_state (Utilities|Casting|CastToBP_MarioGameState (Game|GetGameState)))
  (Variables|/Game/GameModes/BP_MarioGameState.BP_MarioGameState_C|Setplayer%20Hammer _asbp_mario_game_state self))

(event Collision|EventActorBeginOverlap
  (params (OtherActor :type Actor%20Object%20Reference)))

(event EventTick
  (params (DeltaSeconds :type Float%20%28single-precision%29))
  (CallFunction|UpdatePosition)
  (CallFunction|UpdateTimeSinceThrown)
  (CallFunction|UpdateRotation)
  (CallFunction|UpdateIdleTime))

(event Input|ActionEvents|InputActionLeftClick
  (params (Key :type Key%20Structure))
  (:Pressed
    (switch Utilities|FlowControl|Switch|SwitchonHammerState (Variables|Default|Getstate)
      (:NewEnumerator0
        (CallFunction|ThrowHammer)))))

(fn ConstructionScript)

(fn UpdatePosition
  (switch Utilities|FlowControl|Switch|SwitchonHammerState (Variables|Default|Getstate)
    (:NewEnumerator0
      (CallFunction|SetLocationtoPlayer))
    (:NewEnumerator1
      (CallFunction|ApplyVelocity))
    (:NewEnumerator2
      (CallFunction|TrackPlayerPosition))))

(fn ThrowHammer
  (bind _returnvalue (Utilities|GetPlayertoMouseVector))
  (Variables|Default|Setvelocity (Math|Vector|MakeVector 0.0 (.x _returnvalue) (.y _returnvalue)))
  (Variables|Default|Setstate "NewEnumerator1")
  (Variables|Default|SettimeIdle 0.0))

(fn HandlePlayerCollision
  (params (player :type BP%20Mario%20Object%20Reference))
  (if (Utilities|Enum|Equal(Enum) (Variables|Default|Getstate) "NewEnumerator2")
    (Variables|Default|Setstate "NewEnumerator0")
    (Transformation|SetActorRotation "0, 0, 0")
    (Variables|Default|SettimeSInceThrown 0.0)))

(fn HandleObjectCollision
  (if (Utilities|Enum|Equal(Enum) (Variables|Default|Getstate) "NewEnumerator1")
    (Variables|Default|Setstate "NewEnumerator2")
    ;[1 1 1] Bug fix when hammer hits the wall and is inside the player
    (if (Collision|IsOverlappingActor (Game|Player|GetPlayerPawn 0) :!class /Script/Engine.Actor)
      (CallFunction|HandlePlayerCollision))))

(fn SetLocationtoPlayer
  (Transformation|SetWorldLocation (Variables|Default|GetDefaultSceneRoot) (Utilities|GetPlayerLocation) false false))

(fn ApplyVelocity
  (Transformation|AddWorldOffset (Variables|Default|GetDefaultSceneRoot) (|(({1CDAB018-4AFD-8C13-1BE3-AE86AB004326}*{DDA033B2-4D80-8CF6-3A6B-0EB8265639A8})*deltaTime) (Utilities|Time|GetWorldDeltaSeconds)) false false))

(fn TrackPlayerPosition
  (bind (_returnvalue_x _returnvalue_y) (Utilities|GetHammertoPlayerVector))
  (Variables|Default|Setvelocity (Math|Vector|MakeVector 0.0 _returnvalue_x _returnvalue_y))
  (CallFunction|ApplyVelocity))

(fn UpdateTimeSinceThrown
  ;[1 1 1] check if hammer is outgoing
  (if (Utilities|Enum|Equal(Enum) (Variables|Default|Getstate) "NewEnumerator1")
    ;[1 1 1] update timesincethrown
    (Variables|Default|SettimeSInceThrown (+ (Variables|Default|GettimeSInceThrown) (Utilities|Time|GetWorldDeltaSeconds)))
    ;[1 1 1] check if the hammer needs to return
    (if (> (Variables|Default|GettimeSInceThrown) (Variables|Default|GetsecondsBeforeReturn))
      (Variables|Default|Setstate "NewEnumerator2"))))

(fn UpdateRotation
  (if (Utilities|Enum|NotEqual(Enum) (Variables|Default|Getstate) "NewEnumerator0")
    (Transformation|AddActorLocalRotation (Math|Rotator|MakeRotator (Variables|Default|GetrotationSpeed) 0.0 0.0) false false)))

(fn UpdateIdleTime
  (if (Utilities|Enum|Equal(Enum) (Variables|Default|Getstate) "NewEnumerator0")
    (Variables|Default|SettimeIdle (+ (Variables|Default|GettimeIdle) (Utilities|Time|GetWorldDeltaSeconds)))))