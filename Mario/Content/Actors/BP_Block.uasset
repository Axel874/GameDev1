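; BP_Block is a block actor that plays a scale animation when struck by a hammer or by Mario.
; An overlap with BP_Hammer triggers it unless the hammer is in its first enum state, and a component hit from BP_Mario triggers it when the hit normal points almost straight up.
; Both paths share an IsAnimating guard, cleared when the scale timeline finishes, so animations cannot restart mid-play.
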(event `self.ReceiveActorBeginOverlap`
  (params (OtherActor :type "Actor Object Reference"))
  (bind _asbp_hammer (cast `/Game/Characters/BP_Hammer` OtherActor))
  (if (`|EnumInequality` (`/Game/Characters/BP_Hammer.state` _asbp_hammer) "NewEnumerator0")
    (if (not (`self.isAnimating`)) :!label _label
      (set `self.isAnimating` true)
      (`self.Play Hit Animation`))))

(event `self.block.OnComponentHit`
  (params (HitComponent :type "PrimitiveComponent Object Reference") (OtherActor :type "Actor Object Reference") (OtherComp :type "PrimitiveComponent Object Reference") (NormalImpulse :type "Vector Structure") (Hit :type "HitResult Structure (by ref)"))
  (cast `/Game/Characters/BP_Mario` OtherActor)
  (if (> (.z (`.Normal` (`GameplayStatics.BreakHitResult` Hit))) 0.95)
    (goto _label)))

(event `Play Hit Animation`
  (bind (_direction _newtrack_2) (`Timeline|Timeline_0` :!via `PlayFromStart`)
    (:`Update`
      (`SceneComponent.SetWorldScale3D` (`self.block`) (`KismetMathLibrary.Conv_DoubleToVector` _newtrack_2)))
    (:`Finished`
      (set `self.isAnimating` false))))

(fn `UserConstructionScript`)