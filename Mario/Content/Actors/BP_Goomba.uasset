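; BP_Goomba is a Goomba-style actor that patrols back and forth along the world Y axis around its spawn point.
; BeginPlay saves the starting Y and converts StartingDirection into a sign for movement.
; Each Tick offsets the root by direction, speed and delta time, then calls ReverseDirection when the distance from start exceeds Range.
; Overlapping a BP_Hammer destroys it unless the hammer is in its first enum state.
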(event `self.ReceiveBeginPlay`
  (`self.SaveStartingLocation`)
  (`self.ParseStartingDirection`))

(event `self.ReceiveActorBeginOverlap`
  (params (OtherActor :type "Actor Object Reference"))
  (bind _asbp_hammer (cast `/Game/Characters/BP_Hammer` OtherActor))
  (if (`|EnumInequality` (`/Game/Characters/BP_Hammer.state` _asbp_hammer) "NewEnumerator0")
    (`self.K2_DestroyActor`)))

(event `self.ReceiveTick`
  (params (DeltaSeconds :type "Float (single-precision)"))
  (`self.UpdatePosition`)
  (`self.UpdateDirection`))

(fn `ParseStartingDirection`
  (switch `/Game/Enums/Direction` (`self.startingDirection`)
    (:`NewEnumerator0`
      (set `self.direction` -1.0))
    (:`NewEnumerator1`
      (set `self.direction` 1.0))))

(fn `ReverseDirection`
  (`/Engine/EditorBlueprintResources/StandardMacros.NegateFloat` (`self.direction`)))

(fn `SaveStartingLocation`
  (bind (_returnvalue_x _returnvalue_y) (`KismetMathLibrary.BreakVector` (`self.K2_GetActorLocation`)))
  (set `self.yStart` _returnvalue_y))

(fn `UpdateDirection`
  (if (> (`self.GetDistanceToStart`) (`self.range`))
    (`self.ReverseDirection`)))

(fn `UpdatePosition`
  (`SceneComponent.K2_AddWorldOffset` (`self.DefaultSceneRoot`) (`KismetMathLibrary.MakeVector` 0.0 (* (`self.direction`) (`GameplayStatics.GetWorldDeltaSeconds`) (`self.speed`))) false false))

(fn `UserConstructionScript`)