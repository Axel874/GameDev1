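; BP_Block_Question is a question block that releases a mushroom the first time it is hit.
; It extends a parent block's PlayHitAnimation event, calling the parent version on each invocation.
; An IsHit flag limits the reward to once, when the block switches to a dark material and spawns BP_Mushroom above itself.
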(event `self.Play Hit Animation`
  (`parent.Play Hit Animation`)
  (if (not (`self.isHit`))
    (set `self.isHit` true)
    (`PrimitiveComponent.SetMaterial` (`self.block`) 0 "/Game/Materials/M_Dark.M_Dark")
    (`|SpawnActorFromClass` "/Game/Actors/BP_Mushroom.BP_Mushroom_C" (`KismetMathLibrary.MakeTransform` (+ (`self.K2_GetActorLocation`) (0.0 0.0 120.0))) "Undefined" "OverrideRootScale" null null)))

(fn `UserConstructionScript`
  (`parent.UserConstructionScript`))