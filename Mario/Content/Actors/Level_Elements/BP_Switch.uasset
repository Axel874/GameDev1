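; BP_Switch is a level-element switch that toggles a linked Wall actor when a BP_Hammer overlaps it.
; DestroyWall flips the wall's hidden and collision states rather than destroying it, so another hit can reverse the change.
; A Tick-accumulated timer enforces a minimum cooldown between hits, and each accepted hit restarts it and plays a timeline that scales the Switch component as feedback.
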(event `self.ReceiveBeginPlay`
  (set `self.coolDownAcum` (`self.minCoolDown`)))

(event `self.ReceiveActorBeginOverlap`
  (params (OtherActor :type "Actor Object Reference"))
  (cast `/Game/Characters/BP_Hammer` OtherActor)
  (if (> (`self.coolDownAcum`) (`self.minCoolDown`))
    (`self.DestroyWall`)
    (`|ExecutionSequence`
      (:`then_0`
        (set `self.coolDownAcum` 0.0))
      (:`then_1`
        (bind (_direction _newtrack_2) (`Timeline|growth animation` :!via `PlayFromStart`)
          (:`Update`
            (`SceneComponent.SetWorldScale3D` (`self.Switch`) (`KismetMathLibrary.Conv_DoubleToVector` _newtrack_2))))))))

(event `self.ReceiveTick`
  (params (DeltaSeconds :type "Float (single-precision)"))
  (set `self.coolDownAcum` (+ (`GameplayStatics.GetWorldDeltaSeconds`) (`self.coolDownAcum`))))

(fn `DestroyWall`
  (bind _wall (`self.Wall`))
  (bind _wall_2 (`self.Wall`))
  (`self.SetActorHiddenInGame` _wall_2 (not (`Actor.bHidden` _wall_2)))
  (`self.SetActorEnableCollision` _wall (not (`self.GetActorEnableCollision` _wall))))

(fn `UserConstructionScript`)