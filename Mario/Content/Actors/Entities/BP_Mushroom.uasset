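; BP_Mushroom is a mushroom entity that travels sideways along the Y axis in a game with Mario.
; Each Tick offsets its PhysxCollider by Direction and Speed, scaled by world delta time for frame-rate independence.
; A DirectionTrigger overlap flips Direction, except when the other actor is BP_Mario or BP_Hammer.
; The file holds no pickup or damage logic, only this movement.
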(event `self.ReceiveTick`
  (params (DeltaSeconds :type "Float (single-precision)"))
  (`SceneComponent.K2_AddWorldOffset` (`self.physx collider`) (`KismetMathLibrary.MakeVector` 0.0 (* (`self.direction`) (`GameplayStatics.GetWorldDeltaSeconds`) (`self.speed`))) false false))

(event `self.direction trigger.OnComponentBeginOverlap`
  (params (OverlappedComponent :type "PrimitiveComponent Object Reference") (OtherActor :type "Actor Object Reference") (OtherComp :type "PrimitiveComponent Object Reference") (OtherBodyIndex :type Integer) (bFromSweep :type Boolean) (SweepResult :type "HitResult Structure (by ref)"))
  (cast `/Game/Characters/BP_Mario` OtherActor
    (:`CastFailed`
      (cast `/Game/Characters/BP_Hammer` OtherActor
        (:`CastFailed`
          (`/Engine/EditorBlueprintResources/StandardMacros.NegateFloat` (`self.direction`)))))))

(fn `UserConstructionScript`)