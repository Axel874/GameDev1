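; BP_CoolCamera is a camera that follows the first player's pawn on the Y and Z axes while keeping its X position fixed.
; Each tick it measures its offset-adjusted distance to the pawn and adds a per-axis correction to its location.
; Within an axis's deadzone it stays still; beyond it, it moves instantly by the excess, keeping the pawn at the deadzone edge without smoothing.
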(event `self.ReceiveTick`
  (params (DeltaSeconds :type "Float (single-precision)"))
  (bind (_returnvalue_x _returnvalue_y _returnvalue_z) (`KismetMathLibrary.BreakVector` (`self.K2_GetActorLocation`)))
  ;[1 1 1] Retrieve camera corrections according to deadzones
  (bind _correction (`self.GetZaxisCorrection`))
  (bind _correction_2 (`self.GetYAxisCorrection`))
  (`self.K2_SetActorLocation` (`KismetMathLibrary.MakeVector` _returnvalue_x (+ _returnvalue_y _correction_2) (+ _returnvalue_z _correction))))

(fn `Float+-`
  (params (`Float 1` :type "Float (double-precision)") (`Float 2` :type "Float (double-precision)"))
  (returns (Return :type "Float (double-precision)"))
  ;[1 1 1] Adds or substracts from float depending on float sign always getting closer to 0
  (return (- `Float 1` (* (`KismetMathLibrary.SignOfFloat` `Float 1`) `Float 2`))))

(fn `GetDistanceToPlayer`
  (returns (Distance :type "Vector Structure"))
  (return (- (+ (`self.K2_GetActorLocation` self) (`KismetMathLibrary.MakeVector` 0.0 (`self.yOffset`) (`self.zOffset`))) (`self.K2_GetActorLocation` (`GameplayStatics.GetPlayerPawn` 0)))))

(fn `GetYAxisCorrection`
  (returns (Correction :type "Float (double-precision)"))
  (bind _distance (`self.GetDistanceToPlayer`))
  (bind _return (`self.Float+-` (.y _distance) (`self.yDeadzone`))) ; reduce distance by deadzone
  (if (> (`KismetMathLibrary.Abs` (.y _distance)) (`self.yDeadzone`))
    (return (* _return -1.0))
    (else
      (return 0.0))))

(fn `GetZaxisCorrection`
  (returns (Correction :type "Float (double-precision)"))
  (bind _distance (`self.GetDistanceToPlayer`))
  (bind _return (`self.Float+-` (.z _distance) (`self.zDeadzone`))) ; reduce distance by deadzone
  (if (> (`KismetMathLibrary.Abs` (.z _distance)) (`self.zDeadzone`))
    (return (* _return -1.0))
    (else
      (return 0.0))))

(fn `UserConstructionScript`)